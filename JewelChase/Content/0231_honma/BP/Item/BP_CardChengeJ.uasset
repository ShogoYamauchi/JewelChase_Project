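; BP_CardChengeJ is an item actor that awards score when the player character passes through it.
; When an overlap with BP_PlayerCharacter ends, it adds 500 points through BP_ScoreManager and destroys itself.
; Ending an overlap with a BP_DestroyPoint destroys it without scoring.
; Tick is empty, and the up-and-down bobbing logic around a starting height is disconnected and never runs.
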(event EventTick
  (params (DeltaSeconds :type Float%20%28single-precision%29)))

(event Collision|EventActorEndOverlap
  (params (OtherActor :type Actor%20Object%20Reference))
  (Utilities|Casting|CastToBP_DestroyPoint OtherActor
    (:then
      (Actor|DestroyActor))
    (:CastFailed
      (Utilities|Casting|CastToBP_PlayerCharacter OtherActor)
      (bind _returnvalue (Actor|GetActorOfClass "/Game/0231_honma/BP/Stage/BP_ScoreManager.BP_ScoreManager_C"))
      (Class|ScoreManager|AddScore _returnvalue 500)
      (Actor|DestroyActor))))

(fn ConstructionScript)
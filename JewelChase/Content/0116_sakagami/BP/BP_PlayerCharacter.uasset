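; BP_PlayerCharacter is the player character Blueprint, handling a blinking effect on its mesh material.
; BeginPlay creates a dynamic material instance on the mesh's first slot and sets a default color value.
; Each Tick copies OpacityValue from its BlinkingComponent, apparently a C++ variable, into the material's BlinkFloatParameter.
; Unconnected leftover nodes hold an attack montage and a mouse-cursor line trace that never run.
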(event EventBeginPlay
  ;[1 1 1] 動的マテリアルを作る(C++で宣言した変数をマテリアルグラフに持って行くために必要
  (bind _returnvalue (Rendering|Material|CreateDynamicMaterialInstance (Variables|Character|GetMesh) 0 0 "None" :!class /Script/Engine.PrimitiveComponent))
  (Variables|Default|SetMat_Blinking _returnvalue)
  (Variables|Default|SetDefaultColorValue "(R=0.000000,G=0.010000,B=0.000000,A=0.000000)"))

(event Collision|EventActorBeginOverlap
  (params (OtherActor :type Actor%20Object%20Reference)))

(event EventTick
  (params (DeltaSeconds :type Float%20%28single-precision%29))
  (Rendering|Material|SetScalarParameterValueonMaterials (Variables|Character|GetMesh) "BlinkFloatParameter" (Variables|/Script/prototype.BlinkingComponent|GetOpacityValue (Utilities|Array|Get(acopy) (Actor|GetComponentsByClass "/Script/prototype.BlinkingComponent")))))

(event Input|ActionEvents|InputActionClick
  (params (Key :type Key%20Structure :default "None")))

(event Input|MouseEvents|RightMouseButton
  (params (Key :type Key%20Structure :default "None")))

(fn ConstructionScript)